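; PC_Dirk is a player controller that manages the main menu, both on the Menu level and during gameplay.
; BeginPlay on the Menu level or the IA_Menu input creates WB_MainMenu with the matching InGame flag, switching to UI-only input with cursor shown and movement ignored.
; CloseMenu removes all widgets and restores game input.
; SaveGame is unfinished, only creating an SG_Dirk object without writing it.
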(event Custom|Close%20Menu
  (bind _self self)
  ;[1 1 1] Fired when menu is closed, closes it
  (Viewport|RemoveAllWidgets)
  (Input|SetInputModeGameOnly _self false)
  (Variables|/Script/Engine.PlayerController|SetbShowMouseCursor _self false)
  (Input|ResetIgnoreMoveInput _self))

(event Custom|SaveGame
  ;[1 1 1] Saves game (WIP)
  (bind _returnvalue (SaveGame|CreateSaveGameObject "/Game/Core/SG_Dirk.SG_Dirk_C"))
  (Variables|Default|SetSaveGameInstance _returnvalue))

(event Input|EnhancedActionEvents|EnhancedInputActionIA_Menu
  (params (ActionValue :type Boolean) (ElapsedSeconds :type Float%20%28double-precision%29) (TriggeredSeconds :type Float%20%28double-precision%29) (InputAction :type Input%20Action%20Object%20Reference :default "/Game/Input/Default/IA_Menu.IA_Menu"))
  (bind _self self)
  ;[1 1 1] Opens menu when action triggered
  (bind _returnvalue (UserInterface|CreateWidget "/Game/UI/Menu/WB_MainMenu.WB_MainMenu_C" _self true))
  (bind _output_get (Variables|Default|SetMenu _returnvalue))
  (UserInterface|Viewport|AddtoViewport _output_get 0)
  (Input|SetInputModeUIOnly _self _returnvalue "DoNotLock" false)
  (Variables|/Script/Engine.PlayerController|SetbShowMouseCursor _self true)
  (Input|SetIgnoreMoveInput _self true))

(event EventBeginPlay
  (bind _self self)
  ;[1 1 1] Called at begining of the game, checks if the level is menu. If yes, loads the main menu
  (bind _returnvalue (Game|GetCurrentLevelName true))
  (if (Utilities|Enum|Equal(Enum) _returnvalue "Menu")
    (bind _returnvalue_2 (UserInterface|CreateWidget "/Game/UI/Menu/WB_MainMenu.WB_MainMenu_C" _self))
    (bind _output_get (Variables|Default|SetMenu _returnvalue_2))
    (UserInterface|Viewport|AddtoViewport _output_get 0)
    (Input|SetInputModeUIOnly _self _returnvalue_2 "DoNotLock" false)
    (Variables|/Script/Engine.PlayerController|SetbShowMouseCursor _self true)
    (Input|SetIgnoreMoveInput _self true)))

(fn ConstructionScript)